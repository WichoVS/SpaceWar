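; EnemieXD is an enemy with normalized health that takes damage from Projectile_Base hits.
; Both begin and end overlap destroy the projectile, play a hit sound and call DañoBody, which lowers health, shows a HitConfirm widget and calls Muerte to destroy the actor at zero.
; DañoHeadshot deals heavier damage but is only called from unconnected logic.
; PawnSensing detects ThirdPersonCharacter but triggers no behavior.
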(event `self.ReceiveBeginPlay`
  (set `self.health` 1.0))

(event `self.ReceiveActorBeginOverlap`
  (params (OtherActor :type "Actor Object Reference"))
  (bind _asprojectile_base (cast `/Game/Projectiles/Projectile_Base` OtherActor)
    (:`then`
      (`/Game/Projectiles/Projectile_Base.DestroyProjectil` _asprojectile_base)
      (`self.DañoBody`)
      (`GameplayStatics.PlaySound2D` "/Game/Sounds/Weapons/HitSoundEffect.HitSoundEffect" 1.0 1.0 0.0 null null))
    (:`CastFailed`
      (`KismetSystemLibrary.PrintString` "Falló" :!label _label))))

(event `self.ReceiveActorEndOverlap`
  (params (OtherActor :type "Actor Object Reference"))
  (bind _asprojectile_base (cast `/Game/Projectiles/Projectile_Base` OtherActor)
    (:`then`
      (`/Game/Projectiles/Projectile_Base.DestroyProjectil` _asprojectile_base)
      (`self.DañoBody`)
      (`GameplayStatics.PlaySound2D` "/Game/Sounds/Weapons/HitSoundEffect.HitSoundEffect" 1.0 1.0 0.0 null null))
    (:`CastFailed`
      (goto _label))))

(event `self.PawnSensing.OnSeePawn`
  (params (Pawn :type "Pawn Object Reference"))
  (cast `/Game/ThirdPersonBP/Blueprints/ThirdPersonCharacter` Pawn))

(fn `DañoBody`
  (set `self.health` (- (`self.health`) 0.2))
  (bind _returnvalue (`|CreateWidget` "/Game/UI/HitConfirm.HitConfirm_C" (`GameplayStatics.GetPlayerController` 0)))
  (`UserWidget.AddToViewport` _returnvalue 0)
  (if (<= (`self.health`) 0.0)
    (`KismetSystemLibrary.PrintString` "Enemie has been slayed")
    (`self.Muerte`)))

(fn `DañoHeadshot`
  (set `self.health` (- (`self.health`) 0.8))
  (bind _returnvalue (`|CreateWidget` "/Game/UI/HitConfirm.HitConfirm_C" (`GameplayStatics.GetPlayerController` 0)))
  (`UserWidget.AddToViewport` _returnvalue 0)
  (if (<= (`self.health`) 0.0)
    (`KismetSystemLibrary.PrintString` "Enemy Has Been Slayed")
    (`self.Muerte`)))

(fn `Muerte`
  (`self.K2_DestroyActor`))

(fn `UserConstructionScript`)