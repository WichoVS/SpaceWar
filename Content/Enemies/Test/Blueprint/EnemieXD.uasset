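; Test enemy that takes locational damage from Projectile_Base projectiles and is destroyed when its health runs out.
; Separate body and head overlap colliders destroy the incoming projectile, apply damage with a much heavier headshot penalty, and play a hit sound.
; Each damage function also adds a new HitConfirm widget to the first player's viewport and calls Muerte to destroy the actor at zero health.
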(event `self.ReceiveBeginPlay`
  (set `self.health` 1.0))

(event `self.BodyCollider.OnComponentBeginOverlap`
  (params (OverlappedComponent :type "PrimitiveComponent Object Reference") (OtherActor :type "Actor Object Reference") (OtherComp :type "PrimitiveComponent Object Reference") (OtherBodyIndex :type Integer) (bFromSweep :type Boolean) (SweepResult :type "HitResult Structure (by ref)"))
  (bind _asprojectile_base (cast `/Game/Projectiles/Projectile_Base` OtherActor))
  (`/Game/Projectiles/Projectile_Base.DestroyProjectil` _asprojectile_base)
  (`self.DañoBody`)
  (`KismetSystemLibrary.PrintString` "Daño en Cuerpo")
  (`GameplayStatics.PlaySound2D` "/Game/Sounds/EffectsHit/HitSoundEffect.HitSoundEffect" 1.0 1.0 0.0 null null))

(event `self.HeadCollider.OnComponentBeginOverlap`
  (params (OverlappedComponent :type "PrimitiveComponent Object Reference") (OtherActor :type "Actor Object Reference") (OtherComp :type "PrimitiveComponent Object Reference") (OtherBodyIndex :type Integer) (bFromSweep :type Boolean) (SweepResult :type "HitResult Structure (by ref)"))
  (bind _asprojectile_base (cast `/Game/Projectiles/Projectile_Base` OtherActor))
  (`/Game/Projectiles/Projectile_Base.DestroyProjectil` _asprojectile_base)
  (`self.DañoHeadshot`)
  (`KismetSystemLibrary.PrintString` "Daño en Cabeza")
  (`GameplayStatics.PlaySound2D` "/Game/Sounds/EffectsHit/HitSoundEffect.HitSoundEffect" 1.0 1.0 0.0 null null))

(event `self.BodyCollider.OnComponentHit`
  (params (HitComponent :type "PrimitiveComponent Object Reference") (OtherActor :type "Actor Object Reference") (OtherComp :type "PrimitiveComponent Object Reference") (NormalImpulse :type "Vector Structure") (Hit :type "HitResult Structure (by ref)")))

(fn `DañoBody`
  (set `self.health` (- (`self.health`) 0.2))
  (bind _returnvalue (`|CreateWidget` "/Game/UI/HitConfirm.HitConfirm_C" (`GameplayStatics.GetPlayerController` 0)))
  (`UserWidget.AddToViewport` _returnvalue 0)
  (if (<= (`self.health`) 0.0)
    (`KismetSystemLibrary.PrintString` "Enemie has been slayed")
    (`self.Muerte`)))

(fn `DañoHeadshot`
  (set `self.health` (- (`self.health`) 0.8))
  (bind _returnvalue (`|CreateWidget` "/Game/UI/HitConfirm.HitConfirm_C" (`GameplayStatics.GetPlayerController` 0)))
  (`UserWidget.AddToViewport` _returnvalue 0)
  (if (<= (`self.health`) 0.0)
    (`KismetSystemLibrary.PrintString` "Enemy Has Been Slayed")
    (`self.Muerte`)))

(fn `Muerte`
  (`self.K2_DestroyActor`))

(fn `UserConstructionScript`)