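; AK47 weapon Blueprint that fires Projectile_Base from the muzzle socket, with semi and full-auto modes.
; StartFire shoots once or runs a looping timer at a rate derived from DPM until EndFire; SwitchFire toggles the mode.
; Shoot checks ammo and the player's IsFiring, activates muzzle flash and alternates two fire sounds.
; Reload decrements the magazine count, refills ammo after a delay and clears the player's InReloading flag.
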(event `self.ReceiveBeginPlay`
  (`|ExecutionSequence`
    (:`then_0`
      (set `self.shootMode` false)
      (set `self.DPM` 600)
      (set `self.ammo` 30)
      (set `self.fireRate` (/ 60.0 (`KismetMathLibrary.Conv_IntToDouble` (`self.DPM`))))
      (set `self.reloadingTime` 2.2)
      (set `self.switchSoundFire` false))
    (:`then_1`
      (set `self.cartuchos` 1))))

(event `Reload`
  (set `self.cartuchos` (- (`self.cartuchos`) 1))
  (`KismetSystemLibrary.Delay` (`self.reloadingTime`))
  (set `self.ammo` 30)
  (`KismetSystemLibrary.PrintString` "Reloaded")
  (bind _asthird_person_character (cast `/Game/ThirdPersonBP/Blueprints/ThirdPersonCharacter` (`GameplayStatics.GetPlayerCharacter` 0)))
  (set `/Game/ThirdPersonBP/Blueprints/ThirdPersonCharacter.inReloading` false _asthird_person_character))

(event `SwitchFire`
  (set `self.shootMode` (not (`self.shootMode`)))
  (`AudioComponent.Play` (`self.SwitchMode`) 0.0))

(event `EndFire`
  (`KismetSystemLibrary.K2_ClearAndInvalidateTimerHandle` (`self.gunTimer`)))

(event `StartFire`
  (if (`self.shootMode`)
    (bind _returnvalue (`KismetSystemLibrary.K2_SetTimer` null "Shoot" (`self.fireRate`) true))
    (set `self.gunTimer` _returnvalue)
    (else
      (`self.Shoot`))))

(fn `Shoot`
  (bind _asthird_person_character (cast `/Game/ThirdPersonBP/Blueprints/ThirdPersonCharacter` (`GameplayStatics.GetPlayerCharacter` 0)))
  (if (and (> (`self.ammo`) 0) (`/Game/ThirdPersonBP/Blueprints/ThirdPersonCharacter.isFiring` _asthird_person_character))
    (`|SpawnActorFromClass` "/Game/Projectiles/Projectile_Base.Projectile_Base_C" (`SceneComponent.GetSocketTransform` (`self.AK`) "Boca_Gun" "RTS_World") "Undefined" "OverrideRootScale" null null)
    (`|ExecutionSequence`
      (:`then_0`
        (`ActorComponent.SetActive` (`self.PS_MuzzleFlash`) true true))
      (:`then_1`
        (if (`self.switchSoundFire`)
          (`AudioComponent.Play` (`self.FireSound`) 0.0)
          (else
            (`AudioComponent.Play` (`self.FireSound2`) 0.0)))
        (set `self.ammo` (- (`self.ammo`) 1))
        (set `self.switchSoundFire` (not (`self.switchSoundFire`)))))
    (else
      (`KismetSystemLibrary.PrintString` "Recarga no tienes municion"))))

(fn `UserConstructionScript`)